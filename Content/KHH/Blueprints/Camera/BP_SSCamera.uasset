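; Shared co-op camera that gives two players a dynamic split screen, merging into one view when they are close.
; Each tick it projects player positions onto the view plane to derive split angle, split ratio and zoom.
; It positions each player's boom and clip-planed scene capture, feeding viewport-sized render targets.
; A post-process material receives angle and line thickness; the angle can optionally snap to interpolated steps.
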(event EventTick
  (params (DeltaSeconds :type Float%20%28single-precision%29))
  (if (== (Utilities|Array|Length (Variables|Default|GetPlayers)) 2)
    (CallFunction|UpdateCamera DeltaSeconds)
    (CallFunction|UpdateResolution)))

(event EventBeginPlay
  (Utilities|FlowControl|Sequence
    (:then_0
      ;[1 1 1] PostProcessing Split view initialization
      (bind _returnvalue (Rendering|Material|CreateDynamicMaterialInstance "/Game/KHH/Blueprints/Camera/MI_SS.MI_SS" "None" "None" :!class /Script/Engine.KismetMaterialLibrary))
      (bind _output_get (Variables|Default|SetPP%20Material%20Instance _returnvalue))
      (Utilities|Array|Add (Utilities|Struct|BreakWeightedBlendables (Utilities|Struct|BreakPostProcessSettings (Variables|/Script/Engine.CameraComponent|GetPostProcessSettings (Variables|CameraActor|GetCameraComponent)))) (Utilities|Struct|MakeWeightedBlendable 1.0 _output_get)))))

(fn ConstructionScript)

(fn AddPlayer
  (params (Player :type BP%20Split%20Screen%20Character%20Object%20Reference))
  (bind _returnvalue (Utilities|Array|AddUnique (Variables|Default|GetPlayers) 0))
  (if (!= _returnvalue -1)
    (Variables|/Script/Engine.SceneCaptureComponent2D|SetTextureTarget (Variables|/Game/SplitScreenCamera/Blueprints/BP_SplitScreenCharacter.BP_SplitScreenCharacter_C|GetSceneCaptureComponent2D Player) (Utilities|Array|Get(acopy) (Variables|Default|GetTexture%20Targets) _returnvalue))
    (if (== _returnvalue 0)
      (bind _asplayer_controller (Utilities|Casting|CastToPlayerController (Pawn|GetController Player)))
      (Game|Player|SetViewTargetwithBlend _asplayer_controller self 0.0 "VTBlend_Linear" 0.0 false))))

(fn RemovePlayer
  (params (Player :type C%20Player%20Object%20Reference))
  (Utilities|Array|RemoveItem (Variables|Default|GetPlayers) Player))

(fn UpdateCamera
  (params (Delta%20Time :type Float%20%28double-precision%29))
  (bind _returnvalue (Viewport|GetViewportSize))
  (bind _cameracomponent (Variables|CameraActor|GetCameraComponent))
  (bind _players (Variables|Default|GetPlayers))
  (bind _split_angle (Variables|Default|GetSplit%20Angle))
  (bind (_x _y) (Math|Vector2D|BreakVector2D _returnvalue))
  (bind _returnvalue_2 (Math|Vector|GetRightVector _cameracomponent))
  (bind _output (Utilities|Array|Get(acopy) _players))
  (bind _scenecapture2d (Variables|/Script/WAH.CPlayer|GetSceneCapture2D _output))
  (bind _cameraboom (Variables|/Script/WAH.CPlayer|GetCameraBoom _output))
  (bind _fovangle (Variables|/Script/Engine.SceneCaptureComponent2D|GetFOVAngle _scenecapture2d))
  (bind _targetarmlength (Variables|/Script/Engine.SpringArmComponent|GetTargetArmLength _cameraboom))
  (bind _returnvalue_3 (/ _fovangle 2.0))
  (bind _returnvalue_4 (Math|Trig|Tan(Radians) _returnvalue_3))
  (bind _returnvalue_5 (* _returnvalue_4 _targetarmlength))
  (for _array_element (Variables|Default|GetPlayers)
    (Utilities|Array|Add (LocalVariables|GetPlayer%20Locations) (Transformation|GetActorLocation _array_element)))
  (LocalVariables|SetPlayer%20Average (Math|Vector|GetVectorArrayAverage (LocalVariables|GetPlayer%20Locations)))
  (for _array_element_2 (LocalVariables|GetPlayer%20Locations)
    (Utilities|Array|Add (LocalVariables|GetPlayer%20Location%20Projected) (Class|KismetMathLibrary|ProjectPointontoPlane _array_element_2 (LocalVariables|GetPlayer%20Average) (Math|Vector|GetForwardVector (Variables|CameraActor|GetCameraComponent)))))
  (CallFunction|UpdateSplitAngle (* (Class|KismetMathLibrary|DegAcos (Math|Vector|DotProduct (Math|Vector|Normalize (- (Utilities|Array|Get(acopy) (LocalVariables|GetPlayer%20Location%20Projected)) (LocalVariables|GetPlayer%20Average))) _returnvalue_2)) (Math|Float|Sign(Float) (.z (Math|Vector|CrossProduct (Math|Vector|Normalize (- (Utilities|Array|Get(acopy) (LocalVariables|GetPlayer%20Location%20Projected)) (LocalVariables|GetPlayer%20Average))) _returnvalue_2)))) Delta%20Time)
  (Rendering|Material|SetScalarParameterValue (Variables|Default|GetPP%20Material%20Instance) "Angle" (+ (Variables|Default|GetSplit%20Angle) 9e+01) :!class /Script/Engine.MaterialInstanceDynamic)
  (LocalVariables|SetSplit%20Start (* (Class|KismetMathLibrary|Hypotenuse (* _returnvalue_5 (Math|Float|Absolute(Float) (Math|Trig|Cos(Degrees) _split_angle))) (* (Math|Float|Absolute(Float) (Math|Trig|Sin(Degrees) _split_angle)) (* _returnvalue_5 (/ _y _x)))) (Variables|Settings|GetMax%20Distance%20Between%20Players) 0.5))
  (bind _output_get (LocalVariables|SetSplit%20Ratio (/ (Math|Float|Max(Float) (Math|Vector|Distance(Vector) (Utilities|Array|Get(acopy) (LocalVariables|GetPlayer%20Location%20Projected)) (LocalVariables|GetPlayer%20Average)) (Math|Vector|Distance(Vector) (Utilities|Array|Get(acopy) (LocalVariables|GetPlayer%20Location%20Projected) 1) (LocalVariables|GetPlayer%20Average))) (LocalVariables|GetSplit%20Start))))
  (Rendering|Material|SetScalarParameterValue (Variables|Default|GetPP%20Material%20Instance) "Line Thickness" (Math|Float|Clamp(Float) (- _output_get 1.0)) :!class /Script/Engine.MaterialInstanceDynamic)
  (Variables|Zoom|SetArm%20Length (Math|Interpolation|FInterpTo (Variables|Zoom|GetArm%20Length) (+ (Variables|Zoom|GetArm%20Length%20Min) (* (- (Variables|Zoom|GetArm%20Length%20Max) (Variables|Zoom|GetArm%20Length%20Min)) (Math|Float|Clamp(Float) (LocalVariables|GetSplit%20Ratio)))) Delta%20Time (Variables|Zoom|GetZoom%20Speed)))
  (LocalVariables|SetSpread%20Camera%20Angle%20Correction (/ 1.0 (Math|Vector|DotProduct (Math|Vector|Normalize (- (Utilities|Array|Get(acopy) (LocalVariables|GetPlayer%20Locations)) (LocalVariables|GetPlayer%20Average))) (Math|Vector|Normalize (- (Utilities|Array|Get(acopy) (LocalVariables|GetPlayer%20Location%20Projected)) (LocalVariables|GetPlayer%20Average))))))
  (for _index (range 0 1)
    (CallFunction|UpdatePlayerCapture _index (Variables|Zoom|GetArm%20Length) (Transformation|GetWorldRotation (Variables|CameraActor|GetCameraComponent)) (Math|Vector|SelectVector (LocalVariables|GetPlayer%20Average) (+ (Utilities|Array|Get(acopy) (LocalVariables|GetPlayer%20Locations) _index) (* (Math|Vector|Normalize (- (LocalVariables|GetPlayer%20Average) (Utilities|Array|Get(acopy) (LocalVariables|GetPlayer%20Locations) _index))) (LocalVariables|GetSplit%20Start) (LocalVariables|GetSpread%20Camera%20Angle%20Correction))) (<= (LocalVariables|GetSplit%20Ratio) 1.0)) (+ (Variables|Default|GetSplit%20Angle) (Math|Float|SelectFloat 1.8e+02 0.0 (Math|Conversions|ToBoolean(Integer) _index))) (<= (LocalVariables|GetSplit%20Ratio) 1.0))))

(fn UpdateResolution
  (bind _returnvalue (Viewport|GetViewportSize))
  (if (Utilities|Operators|NotEqual(!=) _returnvalue (Variables|Default|GetViewport%20Size) 0.0)
    (bind _output_get (Variables|Default|SetViewport%20Size _returnvalue))
    (Rendering|Material|SetVectorParameterValue (Variables|Default|GetPP%20Material%20Instance) "Resolution" (Utilities|Struct|MakeLinearColor (.X (Math|Vector2D|BreakVector2D _output_get)) (.Y (Math|Vector2D|BreakVector2D _output_get)) 0.0 0.0) :!class /Script/Engine.MaterialInstanceDynamic)
    (for _array_element (Variables|Default|GetTexture%20Targets)
      (Rendering|ResizeRenderTarget2D _array_element (Math|Float|Truncate (.X (Math|Vector2D|BreakVector2D _output_get))) (Math|Float|Truncate (.Y (Math|Vector2D|BreakVector2D _output_get)))))))

(fn UpdatePlayerCapture
  (params (Player%20ID :type Integer) (Arm%20Length :type Float%20%28double-precision%29) (NewRotation :type Rotator) (NewLocation :type Vector) (Angle :type Float%20%28double-precision%29) (arePlayersClose :type Boolean))
  (bind _players (Variables|Default|GetPlayers))
  (bind _returnvalue (not arePlayersClose))
  (bind _output (Utilities|Array|Get(acopy) _players Player%20ID))
  (bind _cameraboom (Variables|/Script/WAH.CPlayer|GetCameraBoom _output))
  (bind _scenecapture2d (Variables|/Script/WAH.CPlayer|GetSceneCapture2D _output))
  (bind _returnvalue_2 (Math|Vector|GetForwardVector _scenecapture2d))
  (bind _returnvalue_3 (Math|Vector|GetRightVector _scenecapture2d))
  (bind _returnvalue_4 (Math|Vector|RotateVectorAroundAxis _returnvalue_3 Angle _returnvalue_2))
  (Variables|/Script/Engine.SpringArmComponent|SetTargetArmLength _cameraboom Arm%20Length)
  (Transformation|SetWorldRotation _cameraboom NewRotation false false)
  (Transformation|SetWorldLocation _cameraboom NewLocation false true)
  (Variables|/Script/Engine.SceneCaptureComponent2D|SetClipPlaneBase _scenecapture2d (- (Transformation|GetWorldLocation _scenecapture2d) (* _returnvalue_4 "")))
  (Variables|/Script/Engine.SceneCaptureComponent2D|SetClipPlaneNormal _scenecapture2d _returnvalue_4)
  (if (== Player%20ID 0)
    (Variables|/Script/Engine.SceneCaptureComponent2D|SetbEnableClipPlane _scenecapture2d (not arePlayersClose))
    (else
      (Variables|/Script/Engine.SceneCaptureComponent|SetbCaptureEveryFrame _scenecapture2d _returnvalue)
      (Variables|/Script/Engine.SceneCaptureComponent2D|SetbEnableClipPlane _scenecapture2d _returnvalue))))

(fn UpdateSplitAngle
  (params (Angle :type Float%20%28double-precision%29) (Delta%20Time :type Float%20%28double-precision%29))
  (bind _step_rotation_steps (Variables|StepRotation|GetStep%20Rotation%20Steps))
  (bind _360 (LocalVariables|Get360))
  (bind _returnvalue (/ _360 _step_rotation_steps))
  (if (Variables|StepRotation|GetDo%20Step%20Rotation)
    (bind _output_get (Variables|Default|SetSplit%20Angle (.roll (Math|Interpolation|RInterpTo (Math|Rotator|MakeRotator (Variables|Default|GetSplit%20Angle) 0.0 0.0) (Math|Rotator|MakeRotator (Math|Rotator|NormalizeAxis (+ (Variables|StepRotation|GetStep%20Rotation%20Starting%20Angle) (* (Math|Float|Round (/ (- (Class|KismetMathLibrary|ClampAxis Angle) (Variables|StepRotation|GetStep%20Rotation%20Starting%20Angle)) _returnvalue)) _returnvalue))) 0.0 0.0) Delta%20Time (Variables|StepRotation|GetStep%20Rotation%20Speed)))))
    (return _output_get)
    (else
      (bind _output_get_2 (Variables|Default|SetSplit%20Angle Angle))
      (return _output_get_2))))