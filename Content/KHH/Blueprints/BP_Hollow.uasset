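; BP_Hollow is an actor that produces an expanding hollow cylinder and destroys itself eight seconds after BeginPlay.
; A fast looping timer fires the boom event, which grows OuterRadius by Speed, derives InnerRadius from it at a fixed offset, then calls GenerateCylinder to rebuild the shape.
; GenerateCylinder is not defined in these graphs, and overlap and Tick are unused.
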(event Custom|boom
  (Variables|Default|SetOuterRadius (+ (Variables|Default|GetOuterRadius) (Variables|Default|GetSpeed)))
  (Variables|Default|SetInnerRadius (- (+ (Variables|Default|GetOuterRadius) (Variables|Default|GetSpeed)) 15.0))
  (Class|CHollowCylinder|GenerateCylinder))

(event EventBeginPlay
  (Utilities|Time|SetTimerbyEvent (delegate Custom|boom) 0.01 true)
  (Utilities|FlowControl|Delay 8.0)
  (Actor|DestroyActor))

(event Collision|EventActorBeginOverlap
  (params (OtherActor :type Actor%20Object%20Reference)))

(event EventTick
  (params (DeltaSeconds :type Float%20%28single-precision%29)))

(fn ConstructionScript)